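; Player-controlled tank Blueprint that wires up camera aiming, firing and the turret and barrel meshes.
; Aim azimuth and elevation axes rotate separate horizontal and vertical components for yaw and pitch, and the Fire action calls Fire.
; The construction script assigns the turret and barrel meshes, and BeginPlay passes both components on through SetBarrelReference and SetTurretReference.
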(event EventBeginPlay
  (Class|Tank|SetBarrelReference (Variables|Default|GetTankBarrel))
  (Class|Tank|SetTurretReference (Variables|Default|GetTankTurret)))

(event Input|ActionEvents|InputActionFire
  (params (Key :type Key%20Structure))
  ;[1 1 1] Firing Input binding
  (:Pressed
    (Class|Tank|Fire)))

(event Input|AxisEvents|InputAxisAimAzimuth
  (params (AxisValue :type Float%20%28single-precision%29))
  ;[1 1 1] Horizontal/veritcal Camera Input Binding
  (Transformation|AddLocalRotation (Variables|Default|GetHorizontalRotation) (Math|Rotator|MakeRotator 0.0 0.0 AxisValue) false false))

(event Input|AxisEvents|InputAxisAimElevation
  (params (AxisValue :type Float%20%28single-precision%29))
  ;[1 1 1] Horizontal/veritcal Camera Input Binding
  (Transformation|AddLocalRotation (Variables|Default|GetVerticalRotation) (Math|Rotator|MakeRotator 0.0 AxisValue 0.0) false false))

(fn ConstructionScript
  (Components|StaticMesh|SetStaticMesh (Variables|Default|GetTankTurret) "/Game/Tank/tank_fbx_Turret.tank_fbx_Turret")
  (Components|StaticMesh|SetStaticMesh (Variables|Default|GetTankBarrel) "/Game/Tank/tank_fbx_Barrel.tank_fbx_Barrel"))